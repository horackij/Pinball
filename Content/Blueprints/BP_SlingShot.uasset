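; BP_SlingShot is a pinball slingshot that kicks the ball away and awards score on contact.
; When a BP_Ball overlaps it, it adds points through Pinball_GameMode and applies a velocity-change impulse opposite the Capsule's forward vector.
; It also plays the SlingBounce timeline, which drives the "Percentout" parameter on the StaticMesh's dynamic material to animate the bounce.
; The construction script creates a dynamic material instance on the Capsule component.
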(event `self.ReceiveActorBeginOverlap`
  (params (OtherActor :type "Actor Object Reference"))
  (bind _asbp_ball (cast `/Game/Blueprints/BP_Ball` OtherActor))
  (bind _aspinball_game_mode (cast `/Game/Blueprints/Pinball_gameMode` (`GameplayStatics.GetGameMode`))
    (:`then`
      (`/Game/Blueprints/Pinball_gameMode.AddScore` _aspinball_game_mode 20.0))
    (:`CastFailed`
      _))
  (`PrimitiveComponent.AddImpulse` (`/Game/Blueprints/BP_Ball.Ball` _asbp_ball) (* (`SceneComponent.GetForwardVector` (`self.Capsule`)) -4500.0) "None" true)
  (bind (_direction _bounce) (`Timeline|SlingBounce` :!via `PlayFromStart`)
    (:`Update`
      (bind _asmaterial_instance_dynamic (cast `MaterialInstanceDynamic` (`PrimitiveComponent.GetMaterial` (`self.StaticMesh`) 2)))
      (`MaterialInstanceDynamic.SetScalarParameterValue` _asmaterial_instance_dynamic "Percentout" _bounce))))

(fn `UserConstructionScript`
  (`PrimitiveComponent.CreateDynamicMaterialInstance` (`self.Capsule`) 2 null "None"))