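; HighScoreSave holds the game's high-score table as an array of score structs, kept in descending order and capped at four entries.
; AddHighScore appends the new entry, calls SortSaveData, then trims the array.
; SortSaveData is a selection sort that repeatedly moves the DetermineHighestScoreValue result into a temporary array, then copies it back.
; DetermineLowestScoreValue similarly finds the minimum but is not called here.
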(fn `AddHighScore`
  (params (NewScore :type "/Game/Blueprints/highScoreStructs Structure"))
  (bind _savestructs (`self.SaveStructs`))
  (`KismetArrayLibrary.Array_Add` (`self.SaveStructs`) NewScore)
  (`self.SortSaveData`)
  (`KismetArrayLibrary.Array_Resize` _savestructs (`KismetMathLibrary.Min` 4 (`KismetArrayLibrary.Array_Length` _savestructs))))

(fn `DetermineHighestScoreValue`
  (returns (HighestScoreStruct :type "/Game/Blueprints/highScoreStructs Structure") (HighestScoreIndex :type Integer))
  (locals (HighestScore :type "Float (double-precision)") (HighestIndex :type Integer))
  (bind _highestindex (`local.HighestIndex`))
  (for (_array_element _array_index) (`self.SaveStructs`)
    (set `self.ArrayElementScoreRef` (`.Score_5_350C8E6C4344149EC469C7A313346ED4` (break `/Game/Blueprints/highScoreStructs` _array_element)))
    (bind _output_get (set `self.ArrayIndexRef` _array_index))
    (if (== _output_get 0)
      (set `local.HighestScore` (`self.ArrayElementScoreRef`))
      (set `local.HighestIndex` (`self.ArrayIndexRef`))
      (elif (> (`self.ArrayElementScoreRef`) (`local.HighestScore`))
        (set `local.HighestScore` (`self.ArrayElementScoreRef`))
        (set `local.HighestIndex` (`self.ArrayIndexRef`)))))
  (return (`|GetArrayItem` (`self.SaveStructs`) _highestindex) _highestindex))

(fn `DetermineLowestScoreValue`
  (returns (LowestScoreStruct :type "/Game/Blueprints/highScoreStructs Structure") (LowestScoreIndex :type Integer))
  (locals (LowestScore :type "Float (double-precision)") (LowestIndex :type Integer))
  (bind _lowestindex (`local.LowestIndex`))
  (for (_array_element _array_index) (`self.SaveStructs`)
    (set `self.ArrayElementScoreRef` (`.Score_5_350C8E6C4344149EC469C7A313346ED4` (break `/Game/Blueprints/highScoreStructs` _array_element)))
    (bind _output_get (set `self.ArrayIndexRef` _array_index))
    (if (== _output_get 0)
      (set `local.LowestScore` (`self.ArrayElementScoreRef`))
      (set `local.LowestIndex` (`self.ArrayIndexRef`))
      (elif (< (`self.ArrayElementScoreRef`) (`local.LowestScore`))
        (set `local.LowestScore` (`self.ArrayElementScoreRef`))
        (set `local.LowestIndex` (`self.ArrayIndexRef`)))))
  (return (`|GetArrayItem` (`self.SaveStructs`) _lowestindex) _lowestindex))

(fn `SortSaveData`
  (locals (TempSaveStrut :type "Array of /Game/Blueprints/highScoreStructs Structure"))
  (while (> (`KismetArrayLibrary.Array_Length` (`self.SaveStructs`)) 0)
    (bind (_highestscorestruct _highestscoreindex) (`self.DetermineHighestScoreValue`))
    (`KismetArrayLibrary.Array_Add` (`local.TempSaveStrut`) _highestscorestruct)
    (`KismetArrayLibrary.Array_Remove` (`self.SaveStructs`) _highestscoreindex))
  (set `self.SaveStructs` (`local.TempSaveStrut`)))